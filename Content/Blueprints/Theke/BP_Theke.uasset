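; BP_Theke is an interactable counter where the player hands in a bound bouquet for a waiting customer's order.
; An overlap box shows a "Place Order" widget when the player carries a bouquet, and interacting snaps it onto the counter.
; Exactly four flowers must match the order's classes, with each match removed from Order to handle duplicates.
; It then destroys the bouquet, clears the customer flag and signals right or wrong.
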(event OnComponentBeginOverlap(OverlapBox)
  (params (OverlappedComponent :type Primitive%20Component%20Object%20Reference) (OtherActor :type Actor%20Object%20Reference) (OtherComp :type Primitive%20Component%20Object%20Reference) (OtherBodyIndex :type Integer) (bFromSweep :type Boolean) (SweepResult :type Hit%20Result%20Structure%20%28by%20ref%29))
  (if (== (Utilities|GetClass (Variables|/Game/Blueprints/Player/BP_Player.BP_Player_C|GetPickedUpActor (Variables|Default|GetAs%20BP%20Player))) "/Game/Blueprints/Blumenstrauß/BP_BoundBouquet.BP_BoundBouquet_C")
    (Rendering|SetVisibility (Variables|Default|GetInteractWidget) true false)))

(event OnComponentEndOverlap(OverlapBox)
  (params (OverlappedComponent :type Primitive%20Component%20Object%20Reference) (OtherActor :type Actor%20Object%20Reference) (OtherComp :type Primitive%20Component%20Object%20Reference) (OtherBodyIndex :type Integer))
  (Rendering|SetVisibility (Variables|Default|GetInteractWidget) false false))

(event Custom|CheckPlacedBouquet
  (bind _order (Variables|Default|GetOrder))
  (Rendering|SetVisibility (Variables|Default|GetInteractWidget) false false)
  (if (== (Utilities|Array|Length (Variables|/Game/Blueprints/Blumenstrauß/BP_BoundBouquet.BP_BoundBouquet_C|GetFlowerArray (Variables|Default|GetPlacedBouquet))) 4)
    (Variables|Default|SetCorrectFlowers 0)
    (for _array_element (Variables|/Game/Blueprints/Blumenstrauß/BP_BoundBouquet.BP_BoundBouquet_C|GetFlowerArray (Variables|Default|GetPlacedBouquet))
      (if (>= (Utilities|Array|FindItem _order (Utilities|GetClass _array_element)) 0)
        (Utilities|Array|RemoveIndex _order (Utilities|Array|FindItem _order (Utilities|GetClass _array_element)))
        (Math|Integer|IncrementInt (Variables|Default|GetCorrectFlowers))))
    (if (== (Variables|Default|GetCorrectFlowers) 4)
      (CallFunction|RightOrder)
      (else
        (CallFunction|WrongOrder)))
    (else
      (CallFunction|WrongOrder))))

(event Custom|WrongOrder
  ;[0.15 0.15 0.15 0.5] call event, npc listens to
  (Development|PrintString "FALSE")
  (Utilities|FlowControl|Delay 0.2)
  (CallFunction|RemoveBouquet)
  (Default|CallOrderWrong))

(event Custom|RemoveBouquet
  (for _array_element (Variables|/Game/Blueprints/Blumenstrauß/BP_BoundBouquet.BP_BoundBouquet_C|GetFlowerArray (Variables|Default|GetPlacedBouquet))
    (Actor|DestroyActor _array_element))
  (Actor|DestroyActor (Variables|Default|GetPlacedBouquet))
  (Variables|Default|SetPlacedBouquet 0)
  (Variables|Default|SetIsCustomerHere? false))

(event Custom|RightOrder
  (Development|PrintString "String")
  (Utilities|FlowControl|Delay 0.2)
  (CallFunction|RemoveBouquet)
  (Default|CallOrderRight))

(event EventBeginPlay
  (bind _asbp_player (Utilities|Casting|CastToBP_Player (Game|Player|GetPlayerPawn 0)))
  (Variables|Default|SetAs%20BP%20Player _asbp_player)
  (bind _asbpw_interaction (Utilities|Casting|CastToBPW_Interaction (UserInterface|GetWidget (Variables|Default|GetInteractWidget))))
  (Variables|/Game/Blueprints/Widgets/BPW_Interaction.BPW_Interaction_C|SetFlowerText _asbpw_interaction "Place Order"))

(event EventInteract
  (params (PlayerCharacter :type BP%20Player%20Object%20Reference))
  (if (Variables|Default|GetIsCustomerHere?)
    (Utilities|IsValid (Variables|/Game/Blueprints/Player/BP_Player.BP_Player_C|GetPickedUpActor PlayerCharacter)
      (:Is%20Valid
        (bind _asbp_bound_bouquet (Utilities|Casting|CastToBP_BoundBouquet (Variables|/Game/Blueprints/Player/BP_Player.BP_Player_C|GetPickedUpActor PlayerCharacter)))
        (bind _output_get (Variables|Default|SetPlacedBouquet _asbp_bound_bouquet))
        (Transformation|DetachFromActor _output_get "KeepRelative" "KeepRelative" "KeepRelative")
        (Transformation|AttachComponentToComponent _output_get (Variables|Default|GetPlacePivot) "None" "SnapToTarget" "KeepRelative" "KeepRelative" true)
        (CallFunction|CheckPlacedBouquet)
        (Variables|/Game/Blueprints/Player/BP_Player.BP_Player_C|SetPickedUpActor PlayerCharacter 0)))))

(fn ConstructionScript)