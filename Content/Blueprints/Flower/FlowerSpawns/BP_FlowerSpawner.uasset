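; BP_FlowerSpawner is an interactable flower source that gives the player a new flower to carry.
; On Interact, if the player is not already carrying an actor, it spawns FlowerClass at the player's pickup pivot and hands it over through PickUpActor.
; The construction script copies FlowerMesh from the FlowerClass defaults onto three display meshes, so the spawner previews the flower type it dispenses.
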(event EventBeginPlay)

(event EventTick
  (params (DeltaSeconds :type Float%20%28single-precision%29)))

(event EventInteract
  (params (PlayerCharacter :type BP%20Player%20Object%20Reference))
  (Utilities|IsValid (Variables|/Game/Blueprints/Player/BP_Player.BP_Player_C|GetPickedUpActor PlayerCharacter)
    (:Is%20Not%20Valid
      (bind _returnvalue (Game|SpawnActorfromClass (Variables|Default|GetFlowerClass) (Transformation|GetWorldTransform (Variables|/Game/Blueprints/Player/BP_Player.BP_Player_C|GetPickUpPivot PlayerCharacter)) "AlwaysSpawn" "MultiplyWithRoot" 0 0))
      (Default|PickUpActor PlayerCharacter _returnvalue))))

(event Collision|EventActorBeginOverlap
  (params (OtherActor :type Actor%20Object%20Reference)))

(fn ConstructionScript
  (bind _flowerclass (Variables|Default|GetFlowerClass))
  (bind _flowermesh (Utilities|GetClassDefaults _flowerclass))
  (Components|StaticMesh|SetStaticMesh (Variables|Default|GetFlower2) _flowermesh)
  (Components|StaticMesh|SetStaticMesh (Variables|Default|GetFlower) _flowermesh)
  (Components|StaticMesh|SetStaticMesh (Variables|Default|GetFlower3) _flowermesh))