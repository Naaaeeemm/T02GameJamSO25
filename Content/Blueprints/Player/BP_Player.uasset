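; Player character that walks, interacts and carries one pickup at a time, with trashing support for flowers and bouquets.
; While moving, a timeline procedurally bobs and tilts the pivots, alternating tilt per cycle, flipping yaw by input direction and triggering footsteps.
; Interact sphere-traces at the capsule, messages InteractionInterface actors and attaches pickups to PickUpPivot.
; Also creates the HUD with a reversed fade and opens the pause menu; TryInteract2 is unused.
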(event Custom|CheckWalk
  (bind _returnvalue (Transformation|GetVelocity))
  (bind _startlocuppivot (Variables|Default|Getstartlocuppivot))
  (bind (_x _y _z) (Math|Vector|BreakVector _startlocuppivot))
  (if (or (> (Math|Float|Absolute(Float) (.x _returnvalue)) 0.0) (> (Math|Float|Absolute(Float) (.y _returnvalue)) 0.0))
    (if (not (Audio|Components|Audio|IsPlaying (Variables|Default|GetTimeline)))
      (Utilities|FlowControl|FlipFlop
        (:A
          (Variables|Default|SetRotationDir 1e+01)
          (bind (_direction _z_loc _rotation) (Timeline|Timeline Play)
            (:Update
              (Transformation|SetRelativeLocation (Variables|Default|GetUpPivot) (Math|Vector|MakeVector _x _y (+ _z (* _z_loc 25.0))) false false)
              (Transformation|SetRelativeRotation (Variables|Default|GetPivot) (Math|Rotator|MakeRotator 0.0 (* _rotation (Variables|Default|GetRotationDir)) (CallFunction|FacingDirection)) false false))
            (:Finished
              (CallFunction|Reset))
            (:footstep
              (CallFunction|Footsteps))))
        (:B
          (Variables|Default|SetRotationDir -1e+01)
          (Timeline|Timeline Play))))))

(event Custom|Reset
  (bind _startlocuppivot (Variables|Default|Getstartlocuppivot))
  (bind (_x _y _z) (Math|Vector|BreakVector _startlocuppivot))
  (bind (_direction _z_loc _rotation) (Timeline|Timeline SetNewTime)
    (:Update
      (Transformation|SetRelativeLocation (Variables|Default|GetUpPivot) (Math|Vector|MakeVector _x _y (+ _z (* _z_loc 25.0))) false false)
      (Transformation|SetRelativeRotation (Variables|Default|GetPivot) (Math|Rotator|MakeRotator 0.0 (* _rotation (Variables|Default|GetRotationDir)) (CallFunction|FacingDirection)) false false))
    (:Finished
      (CallFunction|Reset))
    (:footstep
      (CallFunction|Footsteps))))

(event Input|EnhancedActionEvents|EnhancedInputActionIA_Walk
  (params (ActionValue :type Vector%202D%20Structure) (ElapsedSeconds :type Float%20%28double-precision%29) (TriggeredSeconds :type Float%20%28double-precision%29) (InputAction :type Input%20Action%20Object%20Reference :default "/Game/Input/InputAction/IA_Walk.IA_Walk"))
  ;[0.15 0.15 0.15 0.5] Input
  (Variables|Default|SetDirection (.x ActionValue))
  (Pawn|Input|AddMovementInput (Math|Transform|TransformDirection (Transformation|GetActorTransform) (Math|Vector|MakeVector (.x ActionValue) (.y ActionValue) 0.0)) 1.0 false))

(event Input|EnhancedActionEvents|EnhancedInputActionIA_Interact
  (params (ActionValue :type Boolean) (ElapsedSeconds :type Float%20%28double-precision%29) (TriggeredSeconds :type Float%20%28double-precision%29) (InputAction :type Input%20Action%20Object%20Reference :default "/Game/Input/InputAction/IA_Interact.IA_Interact"))
  ;[0.15 0.15 0.15 0.5] Input
  (CallFunction|TryInteract))

(event Input|EnhancedActionEvents|EnhancedInputActionIA_Pause
  (params (ActionValue :type Boolean) (ElapsedSeconds :type Float%20%28double-precision%29) (TriggeredSeconds :type Float%20%28double-precision%29) (InputAction :type Input%20Action%20Object%20Reference :default "/Game/Input/InputAction/IA_Pause.IA_Pause"))
  ;[0.15 0.15 0.15 0.5] Input
  (CallFunction|OpenPauseMenu))

(event EventBeginPlay
  (Variables|Default|Setstartlocuppivot (Variables|/Script/Engine.SceneComponent|GetRelativeLocation (Variables|Default|GetUpPivot)))
  (bind _returnvalue (UserInterface|CreateWidget "/Game/Blueprints/Widgets/BPW_PlayerInGameHUD.BPW_PlayerInGameHUD_C" (Game|GetPlayerController 0)))
  (bind _output_get (Variables|Default|SetHUDWIdget _returnvalue))
  (UserInterface|Viewport|AddtoPlayerScreen _output_get)
  (Class|UserWidget|PlayAnimationReverse (Variables|Default|GetHUDWIdget) (Variables|/Game/Blueprints/Widgets/BPW_PlayerInGameHUD.BPW_PlayerInGameHUD_C|GetFadeBlack (Variables|Default|GetHUDWIdget)) 1.0 false))

(event EventTick
  (params (DeltaSeconds :type Float%20%28single-precision%29))
  (CallFunction|CheckWalk))

(fn ConstructionScript)

(fn TryInteract
  (bind _capsule (Variables|Default|GetCapsule))
  (bind _returnvalue (Transformation|GetWorldLocation _capsule))
  (bind (_outhit _returnvalue_2) (Collision|SphereTraceForObjects _returnvalue _returnvalue (Components|Capsule|GetScaledCapsuleRadius (Variables|Default|GetCapsule)) (Utilities|Array|MakeArray "ObjectTypeQuery1" "ObjectTypeQuery2" "ObjectTypeQuery3") false 0 "ForDuration"))
  (if _returnvalue_2
    (Utilities|FlowControl|Sequence
      (:then_0
        (if (Utilities|DoesObjectImplementInterface (.HitActor (Collision|BreakHitResult _outhit)) "/Game/Blueprints/InteractionInterface.InteractionInterface_C")
          (Class|InteractionInterface|Interact(Message) (.HitActor (Collision|BreakHitResult _outhit)) self)))
      (:then_1
        (bind _asbp_pick_up_actor (Utilities|Casting|CastToBP_PickUpActor (.HitActor (Collision|BreakHitResult _outhit))))
        (Utilities|IsValid (Variables|Default|GetPickedUpActor)
          (:Is%20Not%20Valid
            (CallFunction|PickUpActor _asbp_pick_up_actor)))))))

(fn TryInteract2
  (bind _sphere_deactivated (Variables|Default|GetSphere-deactivated))
  (bind _outactors (Collision|SphereOverlapActors (Transformation|GetWorldLocation _sphere_deactivated) (Components|Sphere|GetScaledSphereRadius _sphere_deactivated) (Utilities|Array|MakeArray "ObjectTypeQuery1" "ObjectTypeQuery2" "ObjectTypeQuery4" "ObjectTypeQuery3") 0))
  (for _array_element _outactors
    (bind _asbp_interactable (Utilities|Casting|CastToBP_Interactable _array_element))
    (Default|Interact _asbp_interactable)))

(fn PickUpActor
  (params (PickUp :type BP%20Pick%20Up%20Actor%20Object%20Reference))
  (bind _output_get (Variables|Default|SetPickedUpActor PickUp))
  (Default|BePickedUp _output_get)
  (Transformation|AttachComponentToComponent _output_get (Variables|Default|GetPickUpPivot) "None" "SnapToTarget" "SnapToTarget" "KeepWorld" true))

(fn TrashPickUpActor
  (Transformation|DetachFromActor (Variables|Default|GetPickedUpActor) "KeepWorld" "KeepWorld" "KeepWorld")
  (bind _asbp_bound_bouquet (Utilities|Casting|CastToBP_BoundBouquet (Variables|Default|GetPickedUpActor))
    (:then
      (for _array_element (Variables|/Game/Blueprints/Blumenstrauß/BP_BoundBouquet.BP_BoundBouquet_C|GetFlowerArray _asbp_bound_bouquet)
        (Actor|DestroyActor _array_element))
      (Actor|DestroyActor (Variables|Default|GetPickedUpActor)))
    (:CastFailed
      (bind _asbp_main_flower (Utilities|Casting|CastToBP_MainFlower (Variables|Default|GetPickedUpActor)))
      (Actor|DestroyActor _asbp_main_flower)))
  (Variables|Default|SetPickedUpActor 0))

(fn OpenPauseMenu
  (bind _returnvalue (Game|GetPlayerController 0))
  (Utilities|IsValid (Variables|Default|GetPauseMenu)
    (:Is%20Valid
      _)
    (:Is%20Not%20Valid
      (bind _returnvalue_2 (UserInterface|CreateWidget "/Game/Blueprints/Widgets/BPW_PauseMenu.BPW_PauseMenu_C" (Game|GetPlayerController 0)))
      (Variables|Default|SetPauseMenu _returnvalue_2)))
  (UserInterface|Viewport|AddtoViewport (Variables|Default|GetPauseMenu) 0)
  (Default|SelectWidget (Variables|Default|GetPauseMenu) (Variables|/Game/Blueprints/Widgets/BPW_PauseMenu.BPW_PauseMenu_C|GetButton_Continue (Variables|Default|GetPauseMenu)))
  (Variables|/Game/Blueprints/Widgets/BPW_PlayerInGameHUD.BPW_PlayerInGameHUD_C|SetIsGamePaused? (Variables|Default|GetHUDWIdget) true)
  (Variables|/Script/Engine.PlayerController|SetbShowMouseCursor _returnvalue true)
  (Input|SetInputModeUIOnly _returnvalue 0 "DoNotLock" true)
  (Game|SetGamePaused true))

(fn FacingDirection
  (return (select (== (Variables|Default|GetDirection) -1.0) 0.0 1.8e+02)))

(fn Footsteps
  (Audio|PlaySoundatLocation "/Game/Audio/SFX/Walk/SC_Steps.SC_Steps" (Transformation|GetActorLocation) "0, 0, 0" 1.0 1.0 0.0 0 0 0 0))