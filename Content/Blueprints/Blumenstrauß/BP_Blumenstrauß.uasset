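; BP_Blumenstrauß is an interactable flower-placement puzzle piece that takes the flower the player carries.
; Interact checks the carried actor's class and that no flower is stored, then records it before comparing its FlowerNumber to BPBlumenhalter's WantedFlower.
; A match attaches the flower to the holder, signals solved, disables the flower's collision and empties the player's hand.
; IsSolved is a stub that always returns false.
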(event EventInteract
  (params (PlayerCharacter :type BP%20Player%20Object%20Reference))
  (Utilities|IsValid (Variables|/Game/Blueprints/Player/BP_Player.BP_Player_C|GetPickedUpActor PlayerCharacter)
    (:Is%20Valid
      (if (== (Variables|Default|GetAcceptedPickUpClass) (Utilities|GetClass (Variables|/Game/Blueprints/Player/BP_Player.BP_Player_C|GetPickedUpActor PlayerCharacter)))
        (Utilities|IsValid (Variables|Default|GetPlacedFlower)
          (:Is%20Not%20Valid
            (Variables|Default|SetPlacedFlower (Variables|/Game/Blueprints/Player/BP_Player.BP_Player_C|GetPickedUpActor PlayerCharacter))
            (if (Utilities|Enum|Equal(Enum) (Variables|/Game/Blueprints/PickUp/BP_PickUpActor.BP_PickUpActor_C|GetFlowerNumber (Variables|/Game/Blueprints/Player/BP_Player.BP_Player_C|GetPickedUpActor PlayerCharacter)) (Variables|/Game/Blueprints/Blumenstrauß/BP_Blumenhalter.BP_Blumenhalter_C|GetWantedFlower (Variables|Default|GetBP_Blumenhalter)))
              (CallFunction|PlaceFlower (Variables|/Game/Blueprints/Player/BP_Player.BP_Player_C|GetPickedUpActor PlayerCharacter))
              (Variables|/Game/Blueprints/Player/BP_Player.BP_Player_C|SetPickedUpActor PlayerCharacter 0))))))))

(event EventTick
  (params (DeltaSeconds :type Float%20%28single-precision%29)))

(fn ConstructionScript)

(fn PlaceFlower
  (params (Flower :type BP%20Pick%20Up%20Actor%20Object%20Reference))
  (bind _output_get (Variables|Default|SetPlacedFlower Flower))
  (Transformation|AttachComponentToComponent _output_get (Variables|Default|GetBP_Blumenhalter) "None" "KeepRelative" "KeepRelative" "KeepRelative" true)
  (Default|GetPlaced Flower)
  (bind _output_get_2 (Variables|/Game/Blueprints/PickUp/BP_PickUpActor.BP_PickUpActor_C|SetFlowerNumber Flower (Variables|/Game/Blueprints/PickUp/BP_PickUpActor.BP_PickUpActor_C|GetFlowerNumber Flower)))
  (if (CallFunction|IsRightFlower? _output_get_2)
    (Development|PrintString "Right Flower")
    (CallFunction|RightFrameSolved)
    (Collision|SetActorEnableCollision Flower false)))

(fn IsRightFlower?
  (params (Flower%20Number :type EFlower%20Enum :default "NewEnumerator0"))
  (return (Utilities|Enum|Equal(Enum) (Variables|/Game/Blueprints/Blumenstrauß/BP_Blumenhalter.BP_Blumenhalter_C|GetWantedFlower (Variables|Default|GetBP_Blumenhalter)) Flower%20Number)))

(fn RightFrameSolved
  (Default|CallSolved))

(fn IsSolved
  (params (Flower :type EFlower%20Enum :default "NewEnumerator0"))
  (return false Flower))