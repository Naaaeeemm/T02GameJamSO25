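; Pivot component for flower placement that reacts when its referenced Bouquet reports a correctly placed flower.
; On BeginPlay it binds to the Bouquet's RightFlowerPlaced event, whose handler prints the result of CheckChild and clears PlacedFlower.
; CheckChild returns the flower's class if its attach parent actor is not self.
; An unfinished, unconnected loop over the NPC's desired flowers never runs.
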(event Custom|RightFlowerPlaced_Event
  (bind _flowerclass (CallFunction|CheckChild (Variables|/Game/Blueprints/Blumenstrauß/BP_Bouquet.BP_Bouquet_C|GetPlacedFlower (Variables|Default|GetBouquet))))
  (Development|PrintString (Utilities|GetClassDisplayName _flowerclass))
  (Variables|/Game/Blueprints/Blumenstrauß/BP_Bouquet.BP_Bouquet_C|SetPlacedFlower (Variables|Default|GetBouquet) 0))

(event EventBeginPlay
  (bind _bouquet (Variables|Default|GetBouquet))
  (Utilities|IsValid _bouquet
    (:Is%20Valid
      (EventDispatchers|AssignRightFlowerPlaced _bouquet (delegate Custom|RightFlowerPlaced_Event)))))

(fn CheckChild
  (params (PickUp :type BP%20Pick%20Up%20Actor%20Object%20Reference))
  (Utilities|IsValid PickUp
    (:Is%20Valid
      (if (not (== (Actor|GetAttachParentActor PickUp) self))
        (return (Utilities|GetClass PickUp))))))