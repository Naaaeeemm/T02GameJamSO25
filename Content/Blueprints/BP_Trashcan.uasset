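; BP_Trashcan is an interactable trashcan where the player discards the actor they are carrying.
; BeginPlay caches the player pawn and labels the interaction widget "Trashcan" through its FlowerText field.
; Overlapping either cylinder while carrying something shows that widget, and ending an overlap with the player hides it.
; The Interact event calls TrashPickUpActor on the player when a picked-up actor is valid.
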(event OnComponentBeginOverlap(Cylinder)
  (params (OverlappedComponent :type Primitive%20Component%20Object%20Reference) (OtherActor :type Actor%20Object%20Reference) (OtherComp :type Primitive%20Component%20Object%20Reference) (OtherBodyIndex :type Integer) (bFromSweep :type Boolean) (SweepResult :type Hit%20Result%20Structure%20%28by%20ref%29))
  (bind _as_bp_player (Variables|Default|GetAs%20BP%20Player))
  (if (== (stale OnComponentBeginOverlap(Cylinder1) OtherActor) _as_bp_player)
    (Utilities|IsValid (Variables|/Game/Blueprints/Player/BP_Player.BP_Player_C|GetPickedUpActor _as_bp_player)
      (:Is%20Valid
        (Rendering|SetVisibility (Variables|Default|Getinteractionwidget) true false)))))

(event OnComponentEndOverlap(Cylinder)
  (params (OverlappedComponent :type Primitive%20Component%20Object%20Reference) (OtherActor :type Actor%20Object%20Reference) (OtherComp :type Primitive%20Component%20Object%20Reference) (OtherBodyIndex :type Integer))
  (if (== (stale OnComponentEndOverlap(Cylinder1) OtherActor) (Variables|Default|GetAs%20BP%20Player))
    (Rendering|SetVisibility (Variables|Default|Getinteractionwidget) false false)))

(event OnComponentBeginOverlap(Cylinder1)
  (params (OverlappedComponent :type Primitive%20Component%20Object%20Reference) (OtherActor :type Actor%20Object%20Reference) (OtherComp :type Primitive%20Component%20Object%20Reference) (OtherBodyIndex :type Integer) (bFromSweep :type Boolean) (SweepResult :type Hit%20Result%20Structure%20%28by%20ref%29))
  (bind _as_bp_player (Variables|Default|GetAs%20BP%20Player))
  (if (== OtherActor _as_bp_player)
    (Utilities|IsValid (Variables|/Game/Blueprints/Player/BP_Player.BP_Player_C|GetPickedUpActor _as_bp_player)
      (:Is%20Valid
        (Rendering|SetVisibility (Variables|Default|Getinteractionwidget) true false)))))

(event OnComponentEndOverlap(Cylinder1)
  (params (OverlappedComponent :type Primitive%20Component%20Object%20Reference) (OtherActor :type Actor%20Object%20Reference) (OtherComp :type Primitive%20Component%20Object%20Reference) (OtherBodyIndex :type Integer))
  (if (== OtherActor (Variables|Default|GetAs%20BP%20Player))
    (Rendering|SetVisibility (Variables|Default|Getinteractionwidget) false false)))

(event EventBeginPlay
  (bind _asbp_player (Utilities|Casting|CastToBP_Player (Game|Player|GetPlayerPawn 0)))
  (Variables|Default|SetAs%20BP%20Player _asbp_player)
  (bind _asbpw_interaction (Utilities|Casting|CastToBPW_Interaction (UserInterface|GetWidget (Variables|Default|Getinteractionwidget))))
  (Variables|/Game/Blueprints/Widgets/BPW_Interaction.BPW_Interaction_C|SetFlowerText _asbpw_interaction "Trashcan"))

(event EventInteract
  (params (PlayerCharacter :type BP%20Player%20Object%20Reference))
  (Utilities|IsValid (Variables|/Game/Blueprints/Player/BP_Player.BP_Player_C|GetPickedUpActor PlayerCharacter)
    (:Is%20Valid
      (Default|TrashPickUpActor PlayerCharacter))))

(fn ConstructionScript)