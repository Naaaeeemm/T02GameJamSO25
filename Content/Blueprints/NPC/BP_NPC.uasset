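; BP_NPC is a flower shop customer that walks to the counter (BP_Theke) and orders four random flowers.
; A Walk timeline moves it with bob and tilt, then hands the order to the counter and shows its text bubble.
; The counter's right/wrong events update the bubble and reverse the timeline; back at the start, it asks the spawner for the next customer and destroys itself.
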(event Custom|Walk%20Back%20outside
  (bind _startloc (Variables|Default|GetStartLoc))
  (bind _theke (Variables|Default|GetTheke))
  (bind _output_get (Variables|Default|SetIsLeaving true))
  (bind (_direction _location _z_loc _rotation) (Timeline|walk Reverse)
    (:Update
      (Transformation|SetActorLocation (Math|Vector|MakeVector (.x (Math|Vector|Lerp(Vector) _startloc (Transformation|GetWorldLocation (Variables|/Game/Blueprints/Theke/BP_Theke.BP_Theke_C|GetGOAL (Variables|Default|GetTheke))) _location)) (.y (Math|Vector|Lerp(Vector) _startloc (Transformation|GetWorldLocation (Variables|/Game/Blueprints/Theke/BP_Theke.BP_Theke_C|GetGOAL (Variables|Default|GetTheke))) _location)) (+ (* _z_loc 3e+01) (.Z (Math|Vector|BreakVector _startloc)))) false false)
      (Transformation|SetRelativeRotation (Variables|Default|GetPivot) (Math|Rotator|MakeRotator 0.0 (* _rotation 1e+01) (CallFunction|SetNPCFacingDirection)) false false))
    (:Finished
      ;[0.15 0.15 0.15 0.5] test for walking back outside
      (if (Variables|Default|GetIsLeaving)
        (Default|SpawnNextCustomer (Variables|Default|GetSpawner))
        (Utilities|FlowControl|Delay 0.2)
        (Actor|DestroyActor)
        (else
          (Variables|/Game/Blueprints/Theke/BP_Theke.BP_Theke_C|SetOrder _theke (Variables|Default|GetDesiredFlowers))
          (Variables|/Game/Blueprints/Theke/BP_Theke.BP_Theke_C|SetIsCustomerHere? _theke true)
          (Rendering|SetVisibility (Variables|Default|GetWidget) true false))))))

(event Custom|RightOrder
  (CallFunction|WalkBackOutside)
  (Default|OrderText (Variables|Default|GetTextBubbleWidget) true))

(event Custom|WrongOrder
  (CallFunction|WalkBackOutside)
  (Default|OrderText (Variables|Default|GetTextBubbleWidget) false))

(event EventBeginPlay
  (bind _asbp_text_bubble (Utilities|Casting|CastToBP_TextBubble (UserInterface|GetWidget (Variables|Default|GetWidget))))
  (Variables|Default|SetTextBubbleWidget _asbp_text_bubble)
  (CallFunction|SetRandomDesiredFlowers)
  (Variables|Default|SetStartLoc (Transformation|GetWorldLocation (Variables|Transformation|GetRootComponent)))
  (bind _returnvalue (Actor|GetActorOfClass "/Game/Blueprints/Theke/BP_Theke.BP_Theke_C"))
  (bind _output_get (Variables|Default|SetTheke _returnvalue))
  (EventDispatchers|BindEventtoOrderRight _output_get (delegate Custom|RightOrder))
  (EventDispatchers|BindEventtoOrderWrong _output_get (delegate Custom|WrongOrder))
  (bind (_direction _location _z_loc _rotation) (Timeline|walk Play)
    (:Update
      (Transformation|SetActorLocation (Math|Vector|MakeVector (.x (Math|Vector|Lerp(Vector) (Variables|Default|GetStartLoc) (Transformation|GetWorldLocation (Variables|/Game/Blueprints/Theke/BP_Theke.BP_Theke_C|GetGOAL (Variables|Default|GetTheke))) _location)) (.y (Math|Vector|Lerp(Vector) (Variables|Default|GetStartLoc) (Transformation|GetWorldLocation (Variables|/Game/Blueprints/Theke/BP_Theke.BP_Theke_C|GetGOAL (Variables|Default|GetTheke))) _location)) (+ (* _z_loc 3e+01) (.Z (Math|Vector|BreakVector (Variables|Default|GetStartLoc))))) false false)
      (Transformation|SetRelativeRotation (Variables|Default|GetPivot) (Math|Rotator|MakeRotator 0.0 (* _rotation 1e+01) (CallFunction|SetNPCFacingDirection)) false false))
    (:Finished
      ;[0.15 0.15 0.15 0.5] test for walking back outside
      (if (Variables|Default|GetIsLeaving)
        (Default|SpawnNextCustomer (Variables|Default|GetSpawner))
        (Utilities|FlowControl|Delay 0.2)
        (Actor|DestroyActor)
        (else
          (Variables|/Game/Blueprints/Theke/BP_Theke.BP_Theke_C|SetOrder (Variables|Default|GetTheke) (Variables|Default|GetDesiredFlowers))
          (Variables|/Game/Blueprints/Theke/BP_Theke.BP_Theke_C|SetIsCustomerHere? (Variables|Default|GetTheke) true)
          (Rendering|SetVisibility (Variables|Default|GetWidget) true false))))))

(fn ConstructionScript)

(fn SetRandomDesiredFlowers
  (Utilities|Array|Clear (Variables|Default|GetDesiredFlowers))
  (for _index (range 0 3)
    (switch int (Math|Random|RandomIntegerinRange 0 11)
      (:0
        (Utilities|Array|Add (Variables|Default|GetDesiredFlowers) "/Game/Blueprints/Flower/BP_Tulip.BP_Tulip_C")
        (Development|PrintString "Tulip"))
      (:1
        (Utilities|Array|Add (Variables|Default|GetDesiredFlowers) "/Game/Blueprints/Flower/BP_Spiderlily.BP_Spiderlily_C")
        (Development|PrintString "Spider Lily"))
      (:2
        (Utilities|Array|Add (Variables|Default|GetDesiredFlowers) "/Game/Blueprints/Flower/BP_Sunflower.BP_Sunflower_C")
        (Development|PrintString "Sunflower"))
      (:3
        (Utilities|Array|Add (Variables|Default|GetDesiredFlowers) "/Game/Blueprints/Flower/BP_Rose.BP_Rose_C")
        (Development|PrintString "Rose"))
      (:4
        (Utilities|Array|Add (Variables|Default|GetDesiredFlowers) "/Game/Blueprints/Flower/BP_Orchid.BP_Orchid_C")
        (Development|PrintString "Orchid"))
      (:5
        (Utilities|Array|Add (Variables|Default|GetDesiredFlowers) "/Game/Blueprints/Flower/BP_Carnation.BP_Carnation_C")
        (Development|PrintString "Carnation"))
      (:6
        (Utilities|Array|Add (Variables|Default|GetDesiredFlowers) "/Game/Blueprints/Flower/BP_Daffodil.BP_Daffodil_C")
        (Development|PrintString "Daffodil"))
      (:7
        (Utilities|Array|Add (Variables|Default|GetDesiredFlowers) "/Game/Blueprints/Flower/BP_Lily.BP_Lily_C")
        (Development|PrintString "Lily"))
      (:8
        (Utilities|Array|Add (Variables|Default|GetDesiredFlowers) "/Game/Blueprints/Flower/BP_Freesia.BP_Freesia_C")
        (Development|PrintString "Freesia"))
      (:9
        (Utilities|Array|Add (Variables|Default|GetDesiredFlowers) "/Game/Blueprints/Flower/BP_ChristmasRose.BP_ChristmasRose_C")
        (Development|PrintString "Christmas"))
      (:10
        (Utilities|Array|Add (Variables|Default|GetDesiredFlowers) "/Game/Blueprints/Flower/BP_CallaVermeer.BP_CallaVermeer_C")
        (Development|PrintString "Calla Vermeer"))
      (:11
        (Utilities|Array|Add (Variables|Default|GetDesiredFlowers) "/Game/Blueprints/Flower/BP_BlueBell.BP_BlueBell_C")
        (Development|PrintString "BlueBell"))))
  (return))

(fn IsBouquetCorrect?
  (params (Bouquet :type BP%20Bouquet%20Object%20Reference))
  (LocalVariables|SetTMPFLower (Variables|/Game/Blueprints/Blumenstrauß/BP_Bouquet.BP_Bouquet_C|GetFlowers Bouquet))
  (for _array_element (Variables|Default|GetDesiredFlowers)
    (Variables|Default|SetFoundDesiredFlower false)
    (bind _array_element_2 (Utilities|Array|ForEachLoopwithBreak (LocalVariables|GetTMPFLower) :!label _label)
      (:LoopBody
        (if (== (Utilities|GetClass _array_element_2) _array_element)
          (Utilities|Array|RemoveItem (LocalVariables|GetTMPFLower) _array_element_2)
          (Variables|Default|SetFoundDesiredFlower true)
          (goto _label Break)))
      (:Completed
        (if (not (Variables|Default|GetFoundDesiredFlower))
          (return false)))))
  (return true))

(fn SetNPCFacingDirection
  (return (select (Variables|Default|GetIsLeaving) 0.0 1.8e+02)))