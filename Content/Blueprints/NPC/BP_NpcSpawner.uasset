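; NPC spawner that brings customers into the game one at a time, starting a few seconds after play begins.
; Each spawn creates a BP_NPC at the spawner's transform, plays a doorbell sound and hands it spawner and player references.
; The NPC gets a random mesh from an array, and a map keyed by that mesh picks its matching speech.
; The Spawnnextcustomer event repeats the spawn after a short random delay.
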(event Custom|Spawn%20next%20customer
  (Utilities|FlowControl|Delay (Math|Random|RandomFloatinRange 2.5 3.0))
  (bind _returnvalue (Game|SpawnActorfromClass "/Game/Blueprints/NPC/BP_NPC.BP_NPC_C" (Transformation|GetActorTransform) "AlwaysSpawn" "MultiplyWithRoot" 0 0))
  (Audio|PlaySoundatLocation "/Game/Audio/SFX/klingel_tür_game_jam.klingel_tür_game_jam" (Transformation|GetActorLocation) "0, 0, 0" 1.0 1.0 0.0 0 0 0 0)
  (Variables|/Game/Blueprints/NPC/BP_NPC.BP_NPC_C|SetSpawner _returnvalue self)
  (Components|StaticMesh|SetStaticMesh (Variables|/Game/Blueprints/NPC/BP_NPC.BP_NPC_C|GetCube _returnvalue) (.OutItem (Utilities|Array|Random (Variables|Default|GetNPCMeshArray))))
  (Variables|/Game/Blueprints/NPC/BP_NPC.BP_NPC_C|SetPlayer _returnvalue (Variables|Default|GetAs%20BP%20Player))
  (Variables|/Game/Blueprints/NPC/BP_NPC.BP_NPC_C|SetSpeech _returnvalue (.Value (Utilities|Map|Find (Variables|Default|GetSPeechToMesh) (Variables|/Script/Engine.StaticMeshComponent|GetStaticMesh (Variables|/Game/Blueprints/NPC/BP_NPC.BP_NPC_C|GetCube _returnvalue))))))

(event EventBeginPlay
  (bind _asbp_player (Utilities|Casting|CastToBP_Player (Game|Player|GetPlayerPawn 0)))
  (Variables|Default|SetAs%20BP%20Player _asbp_player)
  (Utilities|FlowControl|Delay 4.0)
  (bind _returnvalue (Game|SpawnActorfromClass "/Game/Blueprints/NPC/BP_NPC.BP_NPC_C" (Transformation|GetActorTransform) "AlwaysSpawn" "MultiplyWithRoot" 0 0))
  (Audio|PlaySoundatLocation "/Game/Audio/SFX/klingel_tür_game_jam.klingel_tür_game_jam" (Transformation|GetActorLocation) "0, 0, 0" 1.0 1.0 0.0 0 0 0 0)
  (Variables|/Game/Blueprints/NPC/BP_NPC.BP_NPC_C|SetSpawner _returnvalue self)
  (Components|StaticMesh|SetStaticMesh (Variables|/Game/Blueprints/NPC/BP_NPC.BP_NPC_C|GetCube _returnvalue) (.OutItem (Utilities|Array|Random (Variables|Default|GetNPCMeshArray))))
  (Variables|/Game/Blueprints/NPC/BP_NPC.BP_NPC_C|SetPlayer _returnvalue (Variables|Default|GetAs%20BP%20Player))
  (Variables|/Game/Blueprints/NPC/BP_NPC.BP_NPC_C|SetSpeech _returnvalue (.Value (Utilities|Map|Find (Variables|Default|GetSPeechToMesh) (Variables|/Script/Engine.StaticMeshComponent|GetStaticMesh (Variables|/Game/Blueprints/NPC/BP_NPC.BP_NPC_C|GetCube _returnvalue))))))

(event Collision|EventActorBeginOverlap
  (params (OtherActor :type Actor%20Object%20Reference)))

(event EventTick
  (params (DeltaSeconds :type Float%20%28single-precision%29)))

(fn ConstructionScript)