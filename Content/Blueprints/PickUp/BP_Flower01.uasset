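; BP_Flower01 is a pickup Blueprint for a flower whose look is chosen from twelve variants by a flower number.
; On BeginPlay it calls ChangeFlower with its current number, which stores the value and sets the matching material on the first slot of its static mesh.
; An unconnected mesh-swap node with placeholder basic shapes remains unused.
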(event EventBeginPlay
  (Utilities|FlowControl|Sequence
    (:then_0
      (CallFunction|ChangeFlower (Variables|Default|GetFlowerNumber)))))

(fn ConstructionScript
  (|CallParentFunction))

(fn ChangeFlower
  (params (Flower :type EFlower%20Enum :default "EFlower_MAX"))
  (bind _output_get (Variables|Default|SetFlowerNumber Flower))
  (Rendering|Material|SetMaterial (Variables|Default|GetStaticMesh) 0 (Utilities|Select :Index _output_get :NewEnumerator0 0 :NewEnumerator1 0 :NewEnumerator2 0 :NewEnumerator3 0 :NewEnumerator4 0 :NewEnumerator5 0 :NewEnumerator6 0 :NewEnumerator7 0 :NewEnumerator8 0 :NewEnumerator9 0 :NewEnumerator10 0 :NewEnumerator11 0)))